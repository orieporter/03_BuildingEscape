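; Key actor that snaps into its home volume once it gets near it.
; On the FindHome component's NearHome event, it turns off mesh physics and overlap events.
; A timeline then smoothly lerps location and rotation from the recorded start transform to the home volume's transform, marking FindHome as home when finished.
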(event NearHome(FindHome)
  (bind _staticmeshcomponent (Variables|Debug|GetStaticMeshComponent))
  (bind _findhome (Variables|Default|GetFindHome))
  (bind _homevolume (Variables|/Script/BuildingEscape.FindHome|GetHomeVolume _findhome))
  (Physics|SetSimulatePhysics _staticmeshcomponent false)
  (Variables|/Script/Engine.PrimitiveComponent|SetbGenerateOverlapEvents _staticmeshcomponent false)
  (bind _smooth_motion (Timeline|Timeline_0 Play)
    (:Update
      (Transformation|SetActorLocationAndRotation (Math|Vector|Lerp(Vector) (Variables|/Script/BuildingEscape.FindHome|GetStartLocation _findhome) (Transformation|GetActorLocation _homevolume) _smooth_motion) (Math|Rotator|Lerp(Rotator) (Variables|/Script/BuildingEscape.FindHome|GetStartRotation _findhome) (Transformation|GetActorRotation _homevolume) _smooth_motion)))
    (:Finished
      (Class|FindHome|SetIsHome (Variables|Default|GetFindHome) true))))

(fn ConstructionScript)